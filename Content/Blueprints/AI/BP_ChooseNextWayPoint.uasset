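; Behavior Tree task that sets the next patrol waypoint for an AI-controlled pawn.
; It casts the pawn to ThirdPersonCharacter and caches that character's PatrolPoints array.
; It then uses the Blackboard Index value to pick a point and writes it to the WayPoint key.
; The task only reads the index, never advances it, and always finishes with success.
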(event EventReceiveExecuteAI
  (params (OwnerController :type AI%20Controller%20Object%20Reference) (ControlledPawn :type Pawn%20Object%20Reference))
  ;[1 1 1] Get Patrol Point
  (CallFunction|GetPatrolPoints ControlledPawn)
  ;[1 1 1] Set next way point
  (CallFunction|SetNextWayPoint)
  (AI|BehaviorTree|FinishExecute true))

(fn GetPatrolPoints
  (params (Object :type Object%20Object%20Reference))
  (bind _asthird_person_character (Utilities|Casting|CastToThirdPersonCharacter Object))
  (Variables|Default|SetPatrolPoints (Variables|/Game/ThirdPersonCPP/Blueprints/ThirdPersonCharacter.ThirdPersonCharacter_C|GetPatrolPoints _asthird_person_character)))

(fn SetNextWayPoint
  (Class|BTFunctionLibrary|SetBlackboardValueasObject (Variables|Default|GetWayPoint) (Utilities|Array|Get(acopy) (Variables|Default|GetPatrolPoints) (Class|BTFunctionLibrary|GetBlackboardValueasInt (Variables|Default|GetIndex)))))