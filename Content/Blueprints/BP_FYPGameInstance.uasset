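; BP_FYPGameInstance is a Game Instance that holds the weapon backpack and tracks which weapons the player has selected.
; CanAddWeaponToWeaponSelected counts the selected backpack items and returns that count with whether it is still below MaxSelected.
; SetBackpackItemSelected rebuilds an item struct with a new selection flag and slot, keeping its weapon and image, and writes it back into the array.
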(fn CanAddWeapontoWeaponSelected
  (for _array_element (Variables|Default|GetWeaponBackpackItem)
    (if (.IsSelected (Utilities|Struct|BreakWeaponBackpackItem _array_element))
      (LocalVariables|SetSelectedCount (+ (LocalVariables|GetSelectedCount) 1))))
  (return (LocalVariables|GetSelectedCount) (< (LocalVariables|GetSelectedCount) (Variables|Default|GetMaxSelected))))

(fn SetBackpackItemSelected
  (params (BackPackItemIndex :type Integer) (IsSelected :type Boolean) (WhichSlot :type Integer))
  (bind _weaponbackpackitem (Variables|Default|GetWeaponBackpackItem))
  (bind _item (Utilities|Array|Get(acopy) _weaponbackpackitem BackPackItemIndex))
  (bind (_weapontospawn _backpackimage) (Utilities|Struct|BreakWeaponBackpackItem _item))
  (Utilities|Array|SetArrayElem (Variables|Default|GetWeaponBackpackItem) 0 (Utilities|Struct|MakeWeaponBackpackItem _weapontospawn _backpackimage IsSelected WhichSlot)))