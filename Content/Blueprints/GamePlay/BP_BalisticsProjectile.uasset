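; Ballistic projectile that can penetrate objects, drawing debug lines along its flight path and bounces.
; On bounces faster than MaxPenetration, it destroys itself, spawning a replacement at any exit point found if speed remains.
; Exit search sphere-traces backward through the hit actor, recursing when another object adjoins the far side.
; New speed derives from kinetic energy minus a distance-based loss, though the caller passes a zero vector as exit location.
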(event OnProjectileBounce(ProjectileMovement)
  (params (ImpactResult :type Hit%20Result%20Structure%20%28by%20ref%29) (ImpactVelocity :type Vector%20%28by%20ref%29))
  (bind _newspeed (CallFunction|GetNewSpeed ImpactResult "0, 0, 0" ImpactVelocity))
  ;[1 1 1] Bounce Line
  (Rendering|Debug|DrawDebugLine (Variables|Default|GetLastPosition) (.Location (Collision|BreakHitResult ImpactResult)) "(R=1.000000,G=0.839059,B=0.046377,A=1.000000)" (Variables|Default|GetTraceDuration) 0.0)
  ;[1 1 1] Decide To Penetrate
  (if (> (Math|Vector|VectorLength ImpactVelocity) (Variables|Default|GetMaxPenetration))
    (bind (_exitlocation _resultfound) (CallFunction|ComputeExitLocation ImpactResult ImpactVelocity))
    (if _resultfound
      ;[1 1 1] GetNewSpeed
      (if (> _newspeed 0.0)
        ;[1 1 1] Spawn new projectile
        (bind _returnvalue (Game|SpawnActorfromClass "BP_BalisticsProjectile_C" (Math|Transform|MakeTransform _exitlocation) "Undefined" 0 0))
        (Variables|/Script/Engine.MovementComponent|SetVelocity (Variables|/Script/FYP.Projectile|GetProjectileMovement _returnvalue) (* ImpactVelocity (/ _newspeed (Math|Vector|VectorLength ImpactVelocity))))))
    (Actor|DestroyActor)))

(event EventBeginPlay)

(event Collision|EventActorBeginOverlap
  (params (OtherActor :type Actor%20Object%20Reference)))

(event EventTick
  (params (DeltaSeconds :type Float%20%28single-precision%29))
  (bind _returnvalue (Transformation|GetActorLocation))
  ;[1 1 1] Draw Projectile Line
  (Rendering|Debug|DrawDebugLine (Variables|Default|GetLastPosition) _returnvalue "(R=0.021003,G=1.000000,B=0.000000,A=1.000000)" (Variables|Default|GetTraceDuration) 0.0)
  (Variables|Default|SetLastPosition _returnvalue))

(fn ConstructionScript
  (|CallParentFunction)
  (Variables|Default|SetLastPosition (Transformation|GetActorLocation)))

(fn ComputeExitLocation
  (params (HitResult :type Hit%20Result%20Structure) (ImpactVelosity :type Vector))
  (bind _returnvalue (Math|Vector|Normalize ImpactVelosity))
  (bind (_bblockinghit _binitialoverlap _time _location _impactpoint _normal _impactnormal _physmat _hitactor) (Collision|BreakHitResult HitResult))
  (bind _array (Utilities|Array|MakeArray "ObjectTypeQuery1" "ObjectTypeQuery2" "ObjectTypeQuery3" "ObjectTypeQuery4" "ObjectTypeQuery6"))
  (LocalVariables|SetImpactVelocity ImpactVelosity)
  (bind _outhits (Collision|MultiSphereTraceForObjects (+ (* _returnvalue (Variables|Default|GetDistance)) _location) _location (CallFunction|GetRadius) _array false 0 "None"))
  (if true
    (for _index (range 0 (Utilities|Array|LastIndex _outhits))
      (if (== (.HitActor (Collision|BreakHitResult (Utilities|Array|Get(acopy) _outhits (- (Utilities|Array|LastIndex _outhits) _index)))) _hitactor)
        (bind (_outhit _returnvalue_2) (Collision|SphereTraceForObjects (.Location (Collision|BreakHitResult (Utilities|Array|Get(acopy) _outhits (- (Utilities|Array|LastIndex _outhits) _index)))) (+ _returnvalue (+ (.Location (Collision|BreakHitResult (Utilities|Array|Get(acopy) _outhits (- (Utilities|Array|LastIndex _outhits) _index)))) (.ImpactNormal (Collision|BreakHitResult (Utilities|Array|Get(acopy) _outhits (- (Utilities|Array|LastIndex _outhits) _index)))))) (CallFunction|GetRadius) _array false (Utilities|Array|MakeArray _hitactor) "None"))
        (if _returnvalue_2
          (bind (_exitlocation _resultfound _exitnormal) (CallFunction|ComputeExitLocation _outhit (LocalVariables|GetImpactVelocity)))
          (return _exitlocation _resultfound _exitnormal)
          (else
            (return (.Location (Collision|BreakHitResult (Utilities|Array|Get(acopy) _outhits (- (Utilities|Array|LastIndex _outhits) _index)))) (== (.HitActor (Collision|BreakHitResult (Utilities|Array|Get(acopy) _outhits (- (Utilities|Array|LastIndex _outhits) _index)))) _hitactor) (.ImpactNormal (Collision|BreakHitResult (Utilities|Array|Get(acopy) _outhits (- (Utilities|Array|LastIndex _outhits) _index))))))))))
  ;[1 1 1] No exit
  (return "0, 0, 0" false "0, 0, 0"))

(fn GetRadius
  (return (Variables|/Script/Engine.SphereComponent|GetSphereRadius (Variables|Default|GetCollisionComp))))

(fn GetNewSpeed
  (params (HitResult :type Hit%20Result%20Structure) (ExitLocation :type Vector) (ImpactVelocity :type Vector))
  (return (Math|Float|Sqrt (/ (- (* (Variables|Default|GetMass) (Math|Vector|VectorLengthSquared ImpactVelocity) (LocalVariables|GetScale)) (* (Math|Vector|VectorLength (- ExitLocation (.ImpactPoint (Collision|BreakHitResult HitResult)))) (Variables|Default|GetInitialSpeed))) (* (LocalVariables|GetScale) (Variables|Default|GetMass))))))