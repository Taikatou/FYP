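; Gameplay player controller that handles character spawning, in-game chat and the game-over screen.
; On local BeginPlay it loads saved player settings and passes them toward the server, where the game mode respawns the chosen character, then creates hidden chat and game-over widgets.
; Chat messages fan out through the game mode's controller list, and T toggles the chat window.
; Game over gathers kills and names into leaderboard data and triggers each client's UI.
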(event Custom|PassCharacterInfoToServer
  (params (PlayerSettingsInfo :type Player%20Info%20Structure))
  ;[1 1 1] Pass character info - Respawns player with selected character
  (Variables|Default|SetPlayerSettings PlayerSettingsInfo)
  (bind _asbp_game_play_time_gm (Utilities|Casting|CastToBP_GamePlayTimeGm (Game|GetGameMode)))
  (Default|RespawnPlayer _asbp_game_play_time_gm self (.PlayerCharacter (Utilities|Struct|BreakPlayerInfo (Variables|Default|GetPlayerSettings))) (.PlayerName (Utilities|Struct|BreakPlayerInfo (Variables|Default|GetPlayerSettings))))
  (CallFunction|SetupChatWindow))

(event Custom|SetupChatWindow
  ;[1 1 1] Creates gameplay chat adds to viewport
  (bind _returnvalue (UserInterface|CreateWidget "/Game/Blueprints/UI/AllLevels/GameplayChat.GameplayChat_C"))
  (bind _output_get (Variables|Default|SetGamePlayChat _returnvalue))
  (Widget|SetVisibility _output_get "Hidden")
  (UserInterface|Viewport|AddtoViewport _output_get 0)
  (bind _returnvalue_2 (UserInterface|CreateWidget "/Game/Blueprints/UI/GameOver/GameOverUI.GameOverUI_C"))
  (bind _output_get_2 (Variables|Default|SetGameOverUI _returnvalue_2))
  (UserInterface|Viewport|AddtoViewport _output_get_2 0)
  (Widget|SetVisibility _output_get_2 "Hidden"))

(event Custom|UpdateScoreBoard
  (params (Score :type Integer) (Name :type Text) (Index :type Integer))
  ;[1 1 1] UpdateScoreBoard
  (Default|AddLine (Variables|Default|GetGameOverUI) Score Name Index))

(event Custom|GetChatMessage
  (params (TextToSend :type Text))
  ;[1 1 1] Proccess incoming chat updating clients
  (Variables|Default|SetSendText TextToSend)
  (Variables|Default|SetSenderName (.PlayerName (Utilities|Struct|BreakPlayerInfo (Variables|Default|GetPlayerSettings))))
  (bind _asbp_game_play_time_gm (Utilities|Casting|CastToBP_GamePlayTimeGm (Game|GetGameMode)))
  (for _array_element (Variables|/Game/Blueprints/GamePlay/BP_GamePlayTimeGm.BP_GamePlayTimeGm_C|GetAllPlayerController _asbp_game_play_time_gm)
    (bind _asbp_game_play_player_controller (Utilities|Casting|CastToBP_GamePlayPlayerController _array_element))
    (CallFunction|UpdateChat _asbp_game_play_player_controller (Variables|Default|GetSenderName) (Variables|Default|GetSendText))))

(event Custom|GameOverServer
  ;[1 1 1] GameOverServer
  (bind _asbp_game_play_time_gm (Utilities|Casting|CastToBP_GamePlayTimeGm (Game|GetGameMode)))
  (Utilities|Array|Clear (Variables|Default|GetLeaderBoardData))
  (for _array_element (Variables|/Game/Blueprints/GamePlay/BP_GamePlayTimeGm.BP_GamePlayTimeGm_C|GetAllPlayerController _asbp_game_play_time_gm)
    (bind _asbp_game_play_player_controller (Utilities|Casting|CastToBP_GamePlayPlayerController _array_element))
    (Utilities|Array|Add (Variables|Default|GetLeaderBoardData) (Utilities|Struct|MakeScoreLineData (Class|GameModePlayerState|GetTotalKills (Class|GamePlayPlayerController|GetGamePlayState _asbp_game_play_player_controller)) (Class|GameModePlayerState|GetName (Class|GamePlayPlayerController|GetGamePlayState _asbp_game_play_player_controller)))))
  (for _array_element_2 (Variables|/Game/Blueprints/GamePlay/BP_GamePlayTimeGm.BP_GamePlayTimeGm_C|GetAllPlayerController _asbp_game_play_time_gm)
    (CallFunction|GameOverClient (stale _asbp_game_play_player_controller))))

(event Custom|UpdateChat
  (params (SenderName :type Text) (SenderText :type Text))
  ;[1 1 1] Update client chat window
  (Default|UpdateChatWindow (Variables|/Game/Blueprints/UI/AllLevels/GameplayChat.GameplayChat_C|GetGamePlayChat (Variables|Default|GetGamePlayChat)) SenderName SenderText))

(event Custom|GameOverClient
  ;[1 1 1] GameOverClient
  (Widget|SetVisibility (Variables|Default|GetGameOverUI) "Visible")
  (Input|SetInputModeUIOnly 0 0 "DoNotLock")
  (Variables|Default|SetbShowMouseCursor true))

(event EventBeginPlay
  ;[1 1 1] Load player info pass to server
  (if (Pawn|IsLocalController)
    (Viewport|RemoveAllWidgets)
    (CallFunction|LoadGame)
    (CallFunction|PassCharacterInfotoServer (Variables|Default|GetPlayerSettings))))

(event Input|KeyboardEvents|T
  (params (Key :type Key%20Structure :default "AnyKey"))
  (bind _self self)
  (bind _gameplaychat (Variables|Default|GetGamePlayChat))
  ;[1 1 1] T to type
  (:Pressed
    (Utilities|FlowControl|FlipFlop
      (:A
        (Variables|Default|SetbShowMouseCursor true)
        (Widget|SetVisibility _gameplaychat "Visible")
        (Input|SetInputModeGameandUI _self 0 "DoNotLock" true))
      (:B
        (Variables|Default|SetbShowMouseCursor false)
        (Widget|SetVisibility _gameplaychat "Hidden")
        (Input|SetInputModeGameOnly _self)))))

(fn ConstructionScript)

(fn LoadGame
  (bind _returnvalue (SaveGame|LoadGamefromSlot (Variables|Default|GetPlayerSettingsSave)))
  (bind _asplayer_save_game (Utilities|Casting|CastToPlayerSaveGame _returnvalue))
  (Variables|Default|SetPlayerSettings (Variables|/Game/Blueprints/AllLevels/PlayerSaveGame.PlayerSaveGame_C|GetS_PlayerInfo _asplayer_save_game)))