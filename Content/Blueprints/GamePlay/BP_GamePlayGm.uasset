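; BP_GamePlayGm is the gameplay game mode that handles player controllers, character spawning and logout.
; Swapped-in controllers get game-only input and are added to a tracked list.
; RespawnPlayer destroys any current pawn, spawns the passed class at a random PlayerStart and possesses it.
; On logout, a BP_GamePlayController is passed to GameInfoInstance's DestroySessionCaller for session teardown.
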(event Custom|RespawnPlayer
  (params (PlayerController :type Player%20Controller%20Object%20Reference) (PlayerClass :type Character%20Class%20Reference))
  (bind _returnvalue (Pawn|GetControlledPawn PlayerController))
  ;[1 1 1] Spawn Character with their selected character from gamelay pc
  (bind _outactors (Actor|GetAllActorsOfClass "/Script/Engine.PlayerStart"))
  (Variables|GameInfo|SetSpawnPoints _outactors)
  (Utilities|IsValid _returnvalue
    (:Is%20Valid
      (Actor|DestroyActor _returnvalue))
    (:Is%20Not%20Valid
      _))
  (bind _returnvalue_2 (Game|SpawnActorfromClass PlayerClass (Transformation|GetActorTransform (Utilities|Array|Get(acopy) (Variables|GameInfo|GetSpawnPoints) (Math|Random|RandomIntegerinRange 0 (- (Utilities|Array|Length (Variables|GameInfo|GetSpawnPoints)) 1)))) "Undefined" 0 0))
  (Pawn|Possess PlayerController _returnvalue_2))

(event EventOnSwapPlayerControllers
  (params (OldPC :type Player%20Controller%20Object%20Reference) (NewPC :type Player%20Controller%20Object%20Reference))
  ;[1 1 1] Track connected player controller
  (Input|SetInputModeGameOnly NewPC)
  (Utilities|Array|Add (Variables|GameInfo|GetAllPlayerController) NewPC))

(event EventOnLogout
  (params (ExitingController :type Controller%20Object%20Reference))
  ;[1 1 1] Event Logout destroy session caller
  (bind _asbp_game_play_controller (Utilities|Casting|CastToBP_GamePlayController ExitingController))
  (Default|DestroySessionCaller (.AsGame%20Info%20Instance (Utilities|Casting|CastToGameInfoInstance (Game|GetGameInstance))) _asbp_game_play_controller))

(fn ConstructionScript)