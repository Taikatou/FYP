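; Weapon Blueprint that plays firing visuals using a hitscan-style trace.
; SpawnEmitter spawns an emitter at the weapon mesh and a TrailFx at the first-person muzzle, passing it the shot's end point.
; CalculateShootInformation traces from the camera within a random spread cone, returning the hit, end point and a muzzle transform.
; A blocking hit spawns the ImpactEffect actor at the impact point with the hit result.
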(event EventSpawnEmitter
  (bind _weaponmesh (Variables|Default|GetWeaponMesh))
  (bind _returnvalue (Transformation|GetSocketTransform _weaponmesh "None" "RTS_World"))
  (Effects|SpawnEmitteratLocation 0 (.location _returnvalue) (.rotation _returnvalue))
  (bind (_projectiletransform _hitresult _endlocation) (CallFunction|CalculateShootInformation (Class|BaseCharacter|GetCamera (.AsBase%20Character (Utilities|Casting|CastToBaseCharacter (Components|GetOwner)))) (Variables|Default|GetWeaponMesh) (Transformation|GetWorldLocation (Variables|Default|GetFP_MuzzleLocation))))
  (bind _returnvalue_2 (Effects|SpawnEmitteratLocation (Variables|Default|GetTrailFx) (Transformation|GetWorldLocation (Variables|Default|GetFP_MuzzleLocation))))
  (Effects|Components|ParticleSystem|SetVectorParameter _returnvalue_2 "None" _endlocation)
  (if (.bBlockingHit (Collision|BreakHitResult _hitresult))
    (Game|SpawnActorfromClass "/Game/Blueprints/GamePlay/Effects/ImpactEffect.ImpactEffect_C" (Math|Transform|MakeTransform (.ImpactPoint (Collision|BreakHitResult _hitresult)) "0, 0, 0" "1,1,1") "Undefined" 0 _hitresult 0)))

(fn ConstructionScript)

(fn CalculateShootInformation
  (params (Camera :type Camera%20Component%20Object%20Reference) (WeaponMesh :type Scene%20Component%20Object%20Reference) (MuzzleLocation :type Vector))
  (Utilities|FlowControl|Sequence
    (:then_0
      (LocalVariables|SetLocalCamera Camera)
      (LocalVariables|SetLocalWeaponMesh WeaponMesh)
      (LocalVariables|SetSpawnLocation MuzzleLocation))
    (:then_1
      (LocalVariables|SetLocalEndLoc (+ (.location (Transformation|GetWorldTransform (LocalVariables|GetLocalCamera))) (* (Class|KismetMathLibrary|RandomUnitVectorinCone (Math|Vector|GetForwardVector (.rotation (Transformation|GetWorldTransform (LocalVariables|GetLocalCamera)))) (Variables|Default|GetSpreadCurrent)) 1e+04)))
      (bind (_outhit _returnvalue) (Collision|LineTraceByChannel (.location (Transformation|GetWorldTransform (LocalVariables|GetLocalCamera))) (+ (.location (Transformation|GetWorldTransform (LocalVariables|GetLocalCamera))) (* (Class|KismetMathLibrary|RandomUnitVectorinCone (Math|Vector|GetForwardVector (.rotation (Transformation|GetWorldTransform (LocalVariables|GetLocalCamera)))) (Variables|Default|GetSpreadCurrent)) 1e+04)) "TraceTypeQuery1" false 0 "None"))
      (if _returnvalue
        (LocalVariables|SetLocalTransform (Math|Transform|MakeTransform (LocalVariables|GetSpawnLocation) (Math|Rotator|FindLookatRotation (LocalVariables|GetSpawnLocation) (.ImpactPoint (Collision|BreakHitResult _outhit)))))
        (LocalVariables|SetLocalEndLoc (.ImpactPoint (Collision|BreakHitResult _outhit)))
        (else
          (LocalVariables|SetLocalTransform (Math|Transform|MakeTransform (LocalVariables|GetSpawnLocation) (Pawn|GetControlRotation (.AsPawn (Utilities|Casting|CastToPawn (Components|GetOwner (LocalVariables|GetLocalCamera)))) :!class /Script/Engine.Pawn))))))
    (:then_2
      (return (LocalVariables|GetLocalTransform) _outhit (LocalVariables|GetLocalEndLoc)))))