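; BP_SniperProjectile is a sniper bullet that can penetrate the object it hits.
; On bounce, ComputeExitLocation sphere-traces backward from a set distance along the impact direction to the hit point.
; It takes the last trace hit as the exit, valid only if that is the same actor.
; A valid exit spawns a new projectile there at half the impact velocity, and the original is always destroyed.
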(event OnProjectileBounce(ProjectileMovement)
  (params (ImpactResult :type Hit%20Result%20Structure%20%28by%20ref%29) (ImpactVelocity :type Vector%20%28by%20ref%29))
  ;[1 1 1] Compute Exit Location
  (bind (_exitlocation _resultfound) (CallFunction|ComputeExitLocation ImpactResult ImpactVelocity))
  (if _resultfound
    (bind _returnvalue (Game|SpawnActorfromClass "BP_SniperProjectile_C" (Math|Transform|MakeTransform _exitlocation) "Undefined" 0 0))
    (Variables|/Script/Engine.MovementComponent|SetVelocity (Variables|/Script/FYP.Projectile|GetProjectileMovement _returnvalue) (* ImpactVelocity 0.5))
    (Development|PrintString "Destroying"))
  (Actor|DestroyActor))

(event EventBeginPlay)

(event Collision|EventActorBeginOverlap
  (params (OtherActor :type Actor%20Object%20Reference)))

(event EventTick
  (params (DeltaSeconds :type Float%20%28single-precision%29)))

(fn ConstructionScript
  (|CallParentFunction))

(fn ComputeExitLocation
  (params (HitResult :type Hit%20Result%20Structure) (ImpactVelosity :type Vector))
  (bind (_bblockinghit _binitialoverlap _time _location _impactpoint _normal _impactnormal _physmat _hitactor) (Collision|BreakHitResult HitResult))
  (bind _outhits (Collision|MultiSphereTraceForObjects (+ (* (Math|Vector|Normalize ImpactVelosity) (Variables|Default|GetDistance)) _location) _location (Variables|/Script/Engine.SphereComponent|GetSphereRadius (Variables|Default|GetCollisionComp)) (Utilities|Array|MakeArray "ObjectTypeQuery1" "ObjectTypeQuery2" "ObjectTypeQuery3" "ObjectTypeQuery4" "ObjectTypeQuery6") false 0 "None"))
  (if true
    (for _index (range 0 (Utilities|Array|LastIndex _outhits))
      (return (.Location (Collision|BreakHitResult (Utilities|Array|Get(acopy) _outhits (- (Utilities|Array|LastIndex _outhits) _index)))) (== (.HitActor (Collision|BreakHitResult (Utilities|Array|Get(acopy) _outhits (- (Utilities|Array|LastIndex _outhits) _index)))) _hitactor)))))