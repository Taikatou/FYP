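; CountDownGM, apparently a game mode, runs a start countdown that holds player input until it finishes.
; On BeginPlay it adds a CountDownWidget to the viewport and disables input on player 0's character.
; A looping one-second Delay decrements CountDown, then restores input and removes the widget at zero.
; GetCountDown exposes the current value.
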(event Custom|InitCountDown
  (bind _returnvalue (Game|GetPlayerController 0))
  (bind _returnvalue_2 (UserInterface|CreateWidget "/Game/Blueprints/UI/Campaign/CountDownWidget.CountDownWidget_C" _returnvalue))
  (UserInterface|Viewport|AddtoViewport _returnvalue_2 0)
  (Input|DisableInput (Game|GetPlayerCharacter 0) _returnvalue)
  (Utilities|FlowControl|Delay 1.0 :!label _label)
  (if (!= (Variables|Default|GetCountDown) 0)
    (Variables|Default|SetCountDown (- (Variables|Default|GetCountDown) 1))
    (goto _label)
    (else
      (Input|EnableInput (Game|GetPlayerCharacter 0) (Game|GetPlayerController 0))
      (Widget|RemovefromParent _returnvalue_2))))

(event EventBeginPlay
  (CallFunction|InitCountDown))

(fn ConstructionScript)

(fn GetCountDown
  (return (Variables|Default|GetCountDown)))