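; Gameplay player controller that hands saved player settings to the game mode and provides in-game text chat.
; On local BeginPlay it loads the save and passes it on so BP_GamePlayGm respawns the player as the selected character, then creates a hidden chat widget.
; Incoming messages go through every controller in the game mode's list to update each chat window.
; T toggles chat visibility, cursor and input mode.
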(event Custom|PassCharacterInfoToServer
  (params (PlayerSettingsInfo :type Player%20Info%20Structure))
  ;[1 1 1] Pass character info - Respawns player with selected character
  (Variables|Default|SetPlayerSettings PlayerSettingsInfo)
  (bind _asbp_game_play_gm (Utilities|Casting|CastToBP_GamePlayGm (Game|GetGameMode)))
  (Default|RespawnPlayer _asbp_game_play_gm self (.PlayerCharacter (Utilities|Struct|BreakPlayerInfo (Variables|Default|GetPlayerSettings))))
  (CallFunction|SetupChatWindow))

(event Custom|SetupChatWindow
  ;[1 1 1] Creates gameplay chat adds to viewport
  (bind _returnvalue (UserInterface|CreateWidget "/Game/Blueprints/UI/AllLevels/GameplayChat.GameplayChat_C"))
  (bind _output_get (Variables|Default|SetGamePlayChat _returnvalue))
  (Widget|SetVisibility _output_get "Hidden")
  (UserInterface|Viewport|AddtoViewport _output_get 0))

(event Custom|GetChatMessage
  (params (TextToSend :type Text))
  ;[1 1 1] Proccess incoming chat updating clients
  (Variables|Default|SetSendText TextToSend)
  (Variables|Default|SetSenderName (.PlayerName (Utilities|Struct|BreakPlayerInfo (Variables|Default|GetPlayerSettings))))
  (bind _asbp_game_play_gm (Utilities|Casting|CastToBP_GamePlayGm (Game|GetGameMode)))
  (for _array_element (Variables|/Game/Blueprints/GamePlay/BP_GamePlayGm.BP_GamePlayGm_C|GetAllPlayerController _asbp_game_play_gm)
    (bind _asbp_game_play_controller (Utilities|Casting|CastToBP_GamePlayController _array_element))
    (CallFunction|UpdateChat _asbp_game_play_controller (Variables|Default|GetSenderName) (Variables|Default|GetSendText))))

(event Custom|UpdateChat
  (params (SenderName :type Text) (SenderText :type Text))
  ;[1 1 1] Update client chat window
  (Default|UpdateChatWindow (Variables|/Game/Blueprints/UI/AllLevels/GameplayChat.GameplayChat_C|GetGamePlayChat (Variables|Default|GetGamePlayChat)) SenderName SenderText))

(event EventBeginPlay
  ;[1 1 1] Load player info pass to server
  (if (Pawn|IsLocalController)
    (Viewport|RemoveAllWidgets)
    (CallFunction|LoadGame)
    (CallFunction|PassCharacterInfotoServer (Variables|Default|GetPlayerSettings))))

(event Input|KeyboardEvents|T
  (params (Key :type Key%20Structure :default "AnyKey"))
  (bind _self self)
  (bind _gameplaychat (Variables|Default|GetGamePlayChat))
  ;[1 1 1] T to type
  (:Pressed
    (Utilities|FlowControl|FlipFlop
      (:A
        (Variables|Default|SetbShowMouseCursor true)
        (Widget|SetVisibility _gameplaychat "Visible")
        (Input|SetInputModeGameandUI _self 0 "DoNotLock" true))
      (:B
        (Variables|Default|SetbShowMouseCursor false)
        (Widget|SetVisibility _gameplaychat "Hidden")
        (Input|SetInputModeGameOnly _self)))))

(fn ConstructionScript)

(fn LoadGame
  (bind _returnvalue (SaveGame|LoadGamefromSlot (Variables|Default|GetPlayerSettingsSave)))
  (bind _asplayer_save_game (Utilities|Casting|CastToPlayerSaveGame _returnvalue))
  (Variables|Default|SetPlayerSettings (Variables|/Game/Blueprints/AllLevels/PlayerSaveGame.PlayerSaveGame_C|GetS_PlayerInfo _asplayer_save_game)))