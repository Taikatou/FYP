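; BP_BombCharacter is a playable bomb character that handles its own death, respawn and firing camera shake.
; On death it resets the controller's kill streak, notifies the controller, disables input and respawns as a new bomb character after a delay.
; Respawning spawns the given class at a random PlayerStart, possesses it and destroys the old pawn.
; The H key reuses this to switch to the sniper character.
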(event Custom|OnDeathServer
  (bind _self self)
  (bind _returnvalue (Pawn|GetController _self))
  (bind (_asgame_play_player_controller _bsuccess) (Utilities|Casting|CastToGamePlayPlayerController _returnvalue))
  (if _bsuccess
    (Class|GamePlayPlayerController|OnDeath _asgame_play_player_controller)
    (Input|DisableInput _self 0)
    (Utilities|FlowControl|Delay 3.0)
    (CallFunction|Death "BP_BombCharacter_C")))

(event Custom|Death
  (params (NewParam :type Character%20Class%20Reference))
  (bind _outactors (Actor|GetAllActorsOfClass "/Script/Engine.PlayerStart"))
  (bind _returnvalue (Game|SpawnActorfromClass NewParam (Transformation|GetActorTransform (Utilities|Array|Get(acopy) _outactors (Math|Random|RandomIntegerinRange 0 (- (Utilities|Array|Length _outactors) 1)))) "Undefined" 0 0))
  (Pawn|Possess (Pawn|GetController self) _returnvalue)
  (Actor|DestroyActor self))

(event EventOnDeath
  (params (PlayerController :type Game%20Play%20Player%20Controller%20Object%20Reference))
  (Class|GamePlayPlayerController|ResetKillStreak (.AsGame%20Play%20Player%20Controller (Utilities|Casting|CastToGamePlayPlayerController (Pawn|GetController self))))
  (CallFunction|OnDeathServer))

(event EventFireEvent
  (Camera|PlayWorldCameraShake "/Game/Blueprints/Characters/BombCharacterCameraShake.BombCharacterCameraShake_C" (Transformation|GetActorLocation) 0.0 5e+02))

(event Input|KeyboardEvents|H
  (params (Key :type Key%20Structure :default "AnyKey"))
  (:Pressed
    (CallFunction|Death "/Game/Blueprints/Characters/BP_SniperCharacter.BP_SniperCharacter_C")
    (Development|PrintString "sniper")))

(fn ConstructionScript)