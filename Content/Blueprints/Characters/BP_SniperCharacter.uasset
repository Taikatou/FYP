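; BP_SniperCharacter is a first-person sniper character that handles scope zoom and respawning as another class.
; One timeline, played forward or reversed, drives camera FOV and the sniper HUD's scope opacity while toggling the crosshair.
; On death it updates game play state, disables input and, after a delay, possesses a new BP_BombCharacter at a random PlayerStart, then destroys itself.
; The H key triggers that swap immediately.
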(event Custom|OnDeathServer
  (bind _self self)
  (bind _returnvalue (Pawn|GetController _self))
  (bind (_asgame_play_player_controller _bsuccess) (Utilities|Casting|CastToGamePlayPlayerController _returnvalue))
  (if _bsuccess
    (Class|GameModePlayerState|OnDeath (Class|GamePlayPlayerController|GetGamePlayState _asgame_play_player_controller))
    (Input|DisableInput _self 0)
    (Utilities|FlowControl|Delay 3.0)
    (CallFunction|Death "/Game/Blueprints/Characters/BP_BombCharacter.BP_BombCharacter_C")))

(event Custom|Death
  (params (NewParam :type Character%20Class%20Reference))
  (bind _outactors (Actor|GetAllActorsOfClass "/Script/Engine.PlayerStart"))
  (bind _returnvalue (Game|SpawnActorfromClass NewParam (Transformation|GetActorTransform (Utilities|Array|Get(acopy) _outactors (Math|Random|RandomIntegerinRange 0 (- (Utilities|Array|Length _outactors) 1)))) "Undefined" 0 0))
  (Pawn|Possess (Pawn|GetController self) _returnvalue)
  (Actor|DestroyActor self))

(event EventShowSniperOverlay
  ;[1 1 1] Sniper Scope
  (Variables|Default|SetDrawCrossHair false)
  (bind (_direction _fov _scopeopacity) (Timeline|ScopeAnimationTimeline Play)
    (:Update
      (Camera|SetFieldOfView (Variables|Default|GetFPSCameraComponent) _fov)
      (bind _asbp_sniper_cross_hair_hud (Utilities|Casting|CastToBP_SniperCrossHairHUD (HUD|GetHUD (Game|GetPlayerController 0))))
      (Class|GameplayHUD|SetDrawCrossHair _asbp_sniper_cross_hair_hud (Variables|Default|GetDrawCrossHair))
      (Variables|/Game/Blueprints/UI/GamePlay/BP_SniperCrossHairHUD.BP_SniperCrossHairHUD_C|SetScopeOpacity _asbp_sniper_cross_hair_hud _scopeopacity))))

(event EventHideSniperOverlay
  ;[1 1 1] Sniper Scope
  (Variables|Default|SetDrawCrossHair true)
  (bind (_direction _fov _scopeopacity) (Timeline|ScopeAnimationTimeline Reverse)
    (:Update
      (Camera|SetFieldOfView (Variables|Default|GetFPSCameraComponent) _fov)
      (bind _asbp_sniper_cross_hair_hud (Utilities|Casting|CastToBP_SniperCrossHairHUD (HUD|GetHUD (Game|GetPlayerController 0))))
      (Class|GameplayHUD|SetDrawCrossHair _asbp_sniper_cross_hair_hud (Variables|Default|GetDrawCrossHair))
      (Variables|/Game/Blueprints/UI/GamePlay/BP_SniperCrossHairHUD.BP_SniperCrossHairHUD_C|SetScopeOpacity _asbp_sniper_cross_hair_hud _scopeopacity))))

(event EventOnDeath
  (params (PlayerController :type Game%20Play%20Player%20Controller%20Object%20Reference))
  (Class|GameModePlayerState|ResetKillStreak (Class|GamePlayPlayerController|GetGamePlayState PlayerController))
  (CallFunction|OnDeathServer))

(event Input|KeyboardEvents|H
  (params (Key :type Key%20Structure :default "AnyKey"))
  (:Pressed
    (CallFunction|Death "/Game/Blueprints/Characters/BP_BombCharacter.BP_BombCharacter_C")
    (Development|PrintString "bomb")))

(fn ConstructionScript)