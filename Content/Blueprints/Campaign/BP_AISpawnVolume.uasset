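; BP_AISpawnVolume is a spawn volume that populates its area with patrolling AI ThirdPersonCharacters.
; SpawnAI loops over a requested amount, spawning each AI at a random point in the volume.
; For each AI it also spawns TargetPoints at random points in the volume and adds them to that pawn's PatrolRoute component.
; A separate PrintSpawn event spawns a ThirdPersonCharacter at a given location, without a patrol route.
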(event EventPrintSpawn
  (params (SpawnLocation :type Vector))
  (Game|SpawnActorfromClass "/Game/ThirdPersonCPP/Blueprints/ThirdPersonCharacter.ThirdPersonCharacter_C" (Math|Conversions|ToTransform(Vector) SpawnLocation) "Undefined" 0 0))

(fn ConstructionScript)

(fn SpawnAI
  (params (Amount :type Integer))
  (for _index (range 0 Amount)
    (bind _returnvalue (AI|SpawnAIFromClass "/Game/ThirdPersonCPP/Blueprints/ThirdPersonCharacter.ThirdPersonCharacter_C" 0 (Class|AISpawnVolume|GetRandomPointinVolume) "0, 0, 0" false))
    (for _index_2 (range 0 3)
      (bind _returnvalue_2 (Game|SpawnActorfromClass "/Script/Engine.TargetPoint" (Math|Conversions|ToTransform(Vector) (Class|AISpawnVolume|GetRandomPointinVolume)) "Undefined" 0 0))
      (Class|PatrolRoute|AddActortoPatrolRoute (Actor|GetComponentbyClass _returnvalue "/Script/FYP.PatrolRoute") _returnvalue_2))))