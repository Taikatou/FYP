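; Campaign game mode that builds the level from chained random tiles, tracks score and handles game over.
; BeginPlay seeds the first tiles: a plain starter, then random GeneratedTileAI variants, each placed at the previous tile's attach transform.
; GameOver saves and submits a new high score through GameInfoInstance or fetches the best scores, then pauses and shows the game-over widget.
; UpdatePlayers refreshes that widget's leaderboard.
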(event Custom|GameOver
  (CallFunction|HighScoreCheck)
  (Game|SetGamePaused true)
  (bind _returnvalue (UserInterface|CreateWidget "/Game/Blueprints/UI/Campaign/CampaignGameOver.CampaignGameOver_C" (Game|GetPlayerController 0)))
  (bind _output_get (Variables|Default|SetGameOverUI _returnvalue))
  (UserInterface|Viewport|AddtoViewport _output_get 0)
  (Variables|Default|SetIsGameOver true))

(event Custom|HighScoreCheck
  (bind _returnvalue (Game|GetGameInstance))
  (bind _score (Variables|Default|GetScore))
  (bind _returnvalue_2 (Math|Conversions|ToFloat(Integer) _score))
  (bind _asgame_info_instance (Utilities|Casting|CastToGameInfoInstance (Game|GetGameInstance)))
  (if (> _returnvalue_2 (Variables|/Game/Blueprints/AllLevels/GameInfoInstance.GameInfoInstance_C|GetHighScore _asgame_info_instance))
    (Default|SetHighScoreSP _asgame_info_instance _returnvalue_2)
    (bind _asgame_info_instance_2 (Utilities|Casting|CastToGameInfoInstance _returnvalue))
    (Default|SendHighScore _asgame_info_instance_2 (Math|Conversions|ToFloat(Integer) (Variables|Default|GetScore)) (Variables|Default|GetLevelID))
    (else
      (bind _asgame_info_instance_3 (Utilities|Casting|CastToGameInfoInstance _returnvalue))
      (Default|GetBestHighScores _asgame_info_instance_3))))

(event Custom|UpdatePlayers
  (Default|UpdateLeaderBoard (Variables|Default|GetGameOverUI)))

(event EventBeginPlay
  (|CallParentFunction)
  (for _index (range 0 2)
    (CallFunction|SpawnTile)))

(fn ConstructionScript)

(fn SpawnTile
  (if (== (Variables|Default|GetTiles) 0)
    (bind _returnvalue (Game|SpawnActorfromClass "/Game/Tiles/GeneratedTile.GeneratedTile_C" (Variables|Default|GetNextTileTransform) "Undefined" 0 0))
    (CallFunction|AttachTile _returnvalue)
    (else
      ;[1 1 1] Generate Random levels
      (switch int (Math|Integer|%(Integer) (Math|Random|RandomInteger 4) 4)
        (:Default
          (bind _returnvalue_2 (Game|SpawnActorfromClass "/Game/Tiles/GeneratedTileAI.GeneratedTileAI_C" (Variables|Default|GetNextTileTransform) "Undefined" 0 0 :!label _label))
          (CallFunction|AttachTile _returnvalue_2))
        (:0
          (goto _label))
        (:1
          (bind _returnvalue_3 (Game|SpawnActorfromClass "/Game/Tiles/GeneratedTileAIChild2.GeneratedTileAIChild2_C" (Variables|Default|GetNextTileTransform) "Undefined" 0 0))
          (CallFunction|AttachTile _returnvalue_3))
        (:2
          (bind _returnvalue_4 (Game|SpawnActorfromClass "/Game/Tiles/GeneratedTileAIChild3.GeneratedTileAIChild3_C" (Variables|Default|GetNextTileTransform) "Undefined" 0 0))
          (CallFunction|AttachTile _returnvalue_4))
        (:3
          (bind _returnvalue_5 (Game|SpawnActorfromClass "/Game/Tiles/GeneratedTileAIChild4.GeneratedTileAIChild4_C" (Variables|Default|GetNextTileTransform) "Undefined" 0 0))
          (CallFunction|AttachTile _returnvalue_5))))))

(fn IncrementScore
  (Variables|Default|SetScore (+ (Variables|Default|GetScore) 1)))

(fn AttachTile
  (params (self2 :type Generated%20Tile%20Object%20Reference))
  (bind _attachtransform (Default|GetAttachLocation self2))
  (Variables|Default|SetNextTileTransform _attachtransform)
  (Variables|Default|SetTiles (+ (Variables|Default|GetTiles) 1)))

(fn GetScore
  (return (Variables|Default|GetScore)))