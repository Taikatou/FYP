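; AI spawn volume that populates itself with a requested number of patrolling NPC characters.
; SpawnActors creates an NPC_AI_Controller and a ThirdPersonCharacter for each NPC at random points in the volume, then has the controller possess the character.
; Before possession, it scatters three TargetPoints in the volume and adds them to the character's PatrolRoute component, giving each NPC its own random route.
; The event graph is unused, so spawning relies on an external call.
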(event EventBeginPlay)

(event Collision|EventActorBeginOverlap
  (params (OtherActor :type Actor%20Object%20Reference)))

(event EventTick
  (params (DeltaSeconds :type Float%20%28single-precision%29)))

(fn ConstructionScript)

(fn SpawnActors
  (params (Number :type Integer))
  (bind _returnvalue (Class|SpawnVolume|GetRandomPointinVolume))
  (bind _returnvalue_2 (Math|Conversions|ToTransform(Vector) _returnvalue))
  (for _index (range 1 Number)
    (bind _returnvalue_3 (Game|SpawnActorfromClass "/Game/Blueprints/AI/NPC_AI_Controller.NPC_AI_Controller_C" _returnvalue_2 "Undefined" 0 0))
    (bind _returnvalue_4 (Game|SpawnActorfromClass "/Game/ThirdPersonCPP/Blueprints/ThirdPersonCharacter.ThirdPersonCharacter_C" _returnvalue_2 "Undefined" 0 0))
    (for _index_2 (range 0 2)
      (bind _returnvalue_5 (Game|SpawnActorfromClass "/Script/Engine.TargetPoint" (Math|Conversions|ToTransform(Vector) (Class|SpawnVolume|GetRandomPointinVolume)) "Undefined" 0 0))
      (Class|PatrolRoute|AddActor (Actor|GetComponentbyClass _returnvalue_4 "/Script/FYP.PatrolRoute") _returnvalue_5))
    (Pawn|Possess _returnvalue_3 _returnvalue_4)))